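; Hemy_BP is an unfinished prototype of procedural foot stepping for a skeletal-mesh creature, covering only the FR foot so far.
; Each tick it calls a step check with empty branches, then traces down from the FRT socket with debug drawing and stores the hit as FRLoc.
; HemyShouldStep holds a 2D socket-to-target distance threshold test that is unused, and nothing moves the foot.
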(event EventTick
  (params (DeltaSeconds :type Float%20%28single-precision%29))
  (Utilities|FlowControl|Sequence
    (:then_0
      (if (Utilities|HemyShouldStep "FR" (Variables|Default|GetFR_Loc))
        _
        (else
          _))
      (bind _out_hit_location (Utilities|LineTrace "FRT"))
      (Variables|Default|SetFR_Loc _out_hit_location))))

(fn ConstructionScript)