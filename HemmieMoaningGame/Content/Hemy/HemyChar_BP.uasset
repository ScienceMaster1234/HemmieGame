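; Six-legged Hemy character that procedurally places its feet and has walk and chase speed events.
; Each Tick runs HemyShouldStep per leg, with middle and back legs gated by the NextFoot result of the leg ahead.
; FootLineTrace casts down from a velocity-led target socket and sideways from the body, preferring the sideways hit when blocked, to update that foot's location.
; HemyShouldStep's socket-distance threshold checks are left unconnected.
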(event Custom|ChaseSpeed
  (Variables|/Script/Engine.CharacterMovementComponent|SetMaxWalkSpeed (Variables|Character|GetCharacterMovement) 4e+03))

(event Custom|WalkSpeed
  (Variables|/Script/Engine.CharacterMovementComponent|SetMaxWalkSpeed (Variables|Character|GetCharacterMovement) 1.5e+03))

(event EventTick
  (params (DeltaSeconds :type Float%20%28single-precision%29))
  (bind (_returnvalue _nextfoot) (Utilities|HemyShouldStep "MR" "MRT"))
  (bind (_returnvalue_2 _nextfoot_2) (Utilities|HemyShouldStep "FR" "FRT"))
  (bind (_returnvalue_3 _nextfoot_3) (Utilities|HemyShouldStep "ML" "MLT"))
  (bind (_returnvalue_4 _nextfoot_4) (Utilities|HemyShouldStep "Fl" "FLT"))
  (Utilities|FlowControl|Sequence
    (:then_0
      (if true
        (if _returnvalue_2
          (bind (_out_hit_location _returnvalue_5 _out_hit_location2) (Utilities|FootLineTrace "FRT" 1.0))
          (if _returnvalue_5
            (Variables|Default|SetFR_Loc _out_hit_location2)
            (else
              (Variables|Default|SetFR_Loc _out_hit_location))))))
    (:then_1
      (if _nextfoot_2
        (if _returnvalue
          (bind (_out_hit_location_2 _returnvalue_6 _out_hit_location2_2) (Utilities|FootLineTrace "MRT" 1.0))
          (if _returnvalue_6
            (Variables|Default|SetMR_Loc _out_hit_location2_2)
            (else
              (Variables|Default|SetMR_Loc _out_hit_location_2))))))
    (:then_2
      (if _nextfoot
        (if (.ReturnValue (Utilities|HemyShouldStep "BR" "BRT"))
          (bind (_out_hit_location_3 _returnvalue_7 _out_hit_location2_3) (Utilities|FootLineTrace "BRT" 1.0))
          (if _returnvalue_7
            (Variables|Default|SetBR_Loc _out_hit_location2_3)
            (else
              (Variables|Default|SetBR_Loc _out_hit_location_3))))))
    (:then_3
      (if true
        (if _returnvalue_4
          (bind (_out_hit_location_4 _returnvalue_8 _out_hit_location2_4) (Utilities|FootLineTrace "FLT" -1.0))
          (if _returnvalue_8
            (Variables|Default|SetFL_Loc _out_hit_location2_4)
            (else
              (Variables|Default|SetFL_Loc _out_hit_location_4))))))
    (:then_4
      (if _nextfoot_4
        (if _returnvalue_3
          (bind (_out_hit_location_5 _returnvalue_9 _out_hit_location2_5) (Utilities|FootLineTrace "MLT" -1.0))
          (if _returnvalue_9
            (Variables|Default|SetML_Loc _out_hit_location2_5)
            (else
              (Variables|Default|SetML_Loc _out_hit_location_5))))))
    (:then_5
      (if _nextfoot_3
        (if (.ReturnValue (Utilities|HemyShouldStep "BL" "BLT"))
          (bind (_out_hit_location_6 _returnvalue_10 _out_hit_location2_6) (Utilities|FootLineTrace "BLT" -1.0))
          (if _returnvalue_10
            (Variables|Default|SetBL_Loc _out_hit_location2_6)
            (else
              (Variables|Default|SetBL_Loc _out_hit_location_6))))))))

(fn ConstructionScript)