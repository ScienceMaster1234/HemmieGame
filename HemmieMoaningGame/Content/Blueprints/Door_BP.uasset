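; Interactable door Blueprint that swings its mesh open or closed around the yaw axis.
; Interact checks IsOpen, sets the timeline play rate from the open or close duration, then calls OpenDoor or CloseDoor.
; One timeline plays forward or in reverse to lerp yaw between the closed and open positions, toggling IsOpen when it finishes.
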(event Custom|OpenDoor
  (bind _door_track (Timeline|OpenDoor_Timeline Play)
    (:Update
      (Transformation|SetRelativeRotation (Variables|Default|GetDoor_SM) (Math|Rotator|MakeRotator 0.0 0.0 (Math|Float|Lerp (Variables|Default|GetClosedPosition) (Variables|Default|GetOpenPosition) _door_track)) false false))
    (:Finished
      (Variables|Default|SetIsOpen? (not (Variables|Default|GetIsOpen?))))))

(event Custom|CloseDoor
  (bind _door_track (Timeline|OpenDoor_Timeline Reverse)
    (:Update
      (Transformation|SetRelativeRotation (Variables|Default|GetDoor_SM) (Math|Rotator|MakeRotator 0.0 0.0 (Math|Float|Lerp (Variables|Default|GetClosedPosition) (Variables|Default|GetOpenPosition) _door_track)) false false))
    (:Finished
      (Variables|Default|SetIsOpen? (not (Variables|Default|GetIsOpen?))))))

(fn ConstructionScript)

(fn Interact
  (params (Interactor :type Character%20Object%20Reference))
  (bind _opendoor_timeline (Variables|Default|GetOpenDoor_Timeline))
  (if (not (Variables|Default|GetIsOpen?))
    (Components|Timeline|SetPlayRate _opendoor_timeline (/ 1.0 (Variables|Default|GetTimeToOpen%20%28s%29)))
    (CallFunction|OpenDoor)
    (else
      (Components|Timeline|SetPlayRate _opendoor_timeline (/ 1.0 (Variables|Default|GetTimeToClose%20%28s%29)))
      (CallFunction|CloseDoor)))
  (return true))